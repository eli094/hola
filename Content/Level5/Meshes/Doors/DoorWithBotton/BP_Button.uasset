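; BP_Button is an interactable button in Level5 that opens numbered doors.
; A box trigger shows an interact prompt while the player character overlaps it and removes it on exit.
; On Interaction, it searches all BP_DoorB actors and calls OpenDoor on those whose door number matches its button number.
; A timeline then slides the button mesh along its local Y axis to animate the press.
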(event `self.Box.OnComponentBeginOverlap`
  (params (OverlappedComponent :type "PrimitiveComponent Object Reference") (OtherActor :type "Actor Object Reference") (OtherComp :type "PrimitiveComponent Object Reference") (OtherBodyIndex :type Integer) (bFromSweep :type Boolean) (SweepResult :type "HitResult Structure (by ref)"))
  (if (== OtherActor (`GameplayStatics.GetPlayerCharacter` 0))
    (`UserWidget.AddToViewport` (`self.InteractPrompt`) 0)
    (cast `/Game/FirstPerson/Blueprints/BP_FirstPersonCharacter` OtherActor)))

(event `self.Box.OnComponentEndOverlap`
  (params (OverlappedComponent :type "PrimitiveComponent Object Reference") (OtherActor :type "Actor Object Reference") (OtherComp :type "PrimitiveComponent Object Reference") (OtherBodyIndex :type Integer))
  (if (== (`GameplayStatics.GetPlayerCharacter` 0) OtherActor)
    (`Widget.RemoveFromParent` (`self.InteractPrompt`))
    (cast `/Game/FirstPerson/Blueprints/BP_FirstPersonCharacter` OtherActor)))

(event `/Game/FirstPerson/UI/BP_Interfaces.Interaction`
  (`KismetSystemLibrary.PrintString` "button")
  (`|ExecutionSequence`
    (:`then_0`
      (bind _outactors (`GameplayStatics.GetAllActorsOfClass` "/Game/Level5/Meshes/Doors/DoorWithBotton/BP_DoorB.BP_DoorB_C"))
      (for _array_element _outactors
        (if (== (`/Game/Level5/Meshes/Doors/DoorWithBotton/BP_DoorB.NumberOfDoor` _array_element) (`self.NumberOfButton`))
          (`/Game/Level5/Meshes/Doors/DoorWithBotton/BP_DoorB.OpenDoor` _array_element))))
    (:`then_1`
      (bind (_direction _movmentofbutton) (`Timeline|T_AnimButton`)
        (:`Update`
          (`SceneComponent.K2_SetRelativeLocation` (`self.Button`) (`KismetMathLibrary.MakeVector` 0.0 _movmentofbutton) false false))))))

(fn `UserConstructionScript`)