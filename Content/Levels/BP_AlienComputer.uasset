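; BP_AlienComputer is an interactable console that drives the wave system in BP_WaveGameMode.
; The first interaction begins waves and later ones start a new wave, with presses locked until the game mode's OnEndWave event re-enables them.
; Once a later press finds the wave number at three or more, the console becomes damageable, and draining its health halts the waves.
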(event `self.ReceiveBeginPlay`
  (bind _asbp_wave_game_mode (cast `/Game/FirstPerson/Blueprints/BP_WaveGameMode` (`GameplayStatics.GetGameMode`)))
  (bind _output_get (set `self.As BP Wave Game Mode` _asbp_wave_game_mode))
  (add `/Game/FirstPerson/Blueprints/BP_WaveGameMode.OnEndWave` _output_get (delegate `ResetActivation`)))

(event `ResetActivation`
  (params (WaveNumber :type Integer))
  (set `self.CanPress` true))

(event `/Game/FirstPerson/UI/BP_Interfaces.Interaction`
  (bind _as_bp_wave_game_mode (`self.As BP Wave Game Mode`))
  (if (`self.CanPress`)
    (set `self.CanPress` false)
    (`KismetSystemLibrary.PrintString` "Computer Activated")
    (if (`self.isFirstTime`)
      (set `self.isFirstTime` false)
      (`/Game/FirstPerson/Blueprints/BP_WaveGameMode.BeginWaves` _as_bp_wave_game_mode)
      (else
        (`/Game/FirstPerson/Blueprints/BP_WaveGameMode.NewWave` _as_bp_wave_game_mode)
        (if (>= (`/Game/FirstPerson/Blueprints/BP_WaveGameMode.WaveNumber` (`self.As BP Wave Game Mode`)) 3)
          (set `self.CanBeDamaged` true)
          (`KismetSystemLibrary.PrintString` "Can Destroy console"))))))

(event `self.ReceiveAnyDamage`
  (params (Damage :type "Float (single-precision)") (DamageType :type "DamageType Object Reference") (InstigatedBy :type "Controller Object Reference") (DamageCauser :type "Actor Object Reference"))
  (if (`self.CanBeDamaged`)
    (bind _output_get (set `self.Health` (- (`self.Health`) Damage)))
    (if (<= _output_get 0)
      (`KismetSystemLibrary.PrintString` "Boom")
      (`/Game/FirstPerson/Blueprints/BP_WaveGameMode.HaltWaves` (`self.As BP Wave Game Mode`)))))

(fn `UserConstructionScript`)